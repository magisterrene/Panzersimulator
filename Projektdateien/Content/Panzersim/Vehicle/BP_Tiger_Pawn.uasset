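; Drivable VR Tiger tank pawn that simulates the driver's station on Chaos wheeled vehicle movement.
; Grabbed levers and wheel run looping timers that track the nearest motion controller to set direction, gear, steering and brakes.
; Pedal functions drive throttle, brake and clutch, with single chain brakes turning the tank.
; Clutchless shifts risk killing the tank against a random threshold, while chain-braking at speed or reversing in high gear kills it outright.
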(event OnGrabbed(LeverGC)
  ;[1 1 1] Direction Lever Control
  (Utilities|Time|SetTimerbyEvent (delegate Custom|MoveDirectionLever) 0.01 true))

(event OnGrabbed(SteeringWheelGC)
  ;[1 1 1] Steering Wheel Control
  (Utilities|Time|SetTimerbyEvent (delegate Custom|RotateWheel) 0.01 true))

(event OnDropped(ChainLeverLeftGC)
  ;[1 1 1] ChainLeverLeft Control
  (Class|KismetSystemLibrary|PauseTimer 0 "MoveChainLeverLeft"))

(event OnGrabbed(GearLeverGC)
  ;[1 1 1] Gear Lever Control
  (Utilities|Time|SetTimerbyEvent (delegate Custom|MoveGearLever) 0.01 true))

(event OnDropped(GearLeverGC)
  ;[1 1 1] Gear Lever Control
  (Class|KismetSystemLibrary|PauseTimer 0 "MoveGearLever")
  (Transformation|SetRelativeRotation (Variables|Default|GetSM_GearLever) (Math|Rotator|MakeRotator 0.0 (Math|Conversions|ToFloat(Integer) (- 70 (* (- (Math|Integer|Absolute(Integer) (Variables|Default|GetGear)) 1) 10))) 0.0) false false))

(event OnGrabbed(SketchbookGC)
  ;[1 1 1] Take Sketchbook
  (bind _asvrpawn (Utilities|Casting|CastToVRPawn (Game|Player|GetPlayerPawn 0)))
  (bind _mc (CallFunction|GetGrabbingMC (Transformation|GetWorldLocation (Variables|Default|GetBP_Sketchfab))))
  (Default|ToggleMenu _asvrpawn (== _mc (Variables|/Game/VRTemplate/Blueprints/VRPawn.VRPawn_C|GetMotionControllerRightGrip _asvrpawn))))

(event OnDropped(SteeringWheelGC)
  ;[1 1 1] Steering Wheel Control
  (Class|KismetSystemLibrary|PauseTimer 0 "RotateWheel"))

(event OnDropped(LeverGC)
  ;[1 1 1] Direction Lever Control
  (Class|KismetSystemLibrary|PauseTimer 0 "MoveDirectionLever")
  (Transformation|SetRelativeRotation (Variables|Default|GetSM_DirectionLever) (Math|Rotator|MakeRotator 0.0 (Math|Conversions|ToFloat(Integer) (* (Variables|Default|GetDirection) -20)) 0.0) false false))

(event OnGrabbed(VisibleGC)
  (bind _mesh (Variables|Character|GetMesh))
  (bind _bvisible (Variables|/Script/Engine.SceneComponent|GetbVisible _mesh))
  (bind _returnvalue (not _bvisible))
  ;[1 1 1] Commander Button (Visibility toggle for all not essential Elements)
  (Rendering|SetVisibility (Variables|Default|GetSM_Sighthatch) _returnvalue false)
  (Rendering|SetVisibility (Variables|Default|GetSM_Driverhatch) _returnvalue false)
  (Rendering|SetVisibility (Variables|Default|GetSM_Sightframe) _returnvalue false)
  (Rendering|SetVisibility (Variables|Default|GetSM_Seatblock) _returnvalue true)
  (Rendering|SetVisibility (Variables|Default|Getindustrial_wall_light) _returnvalue false)
  (Rendering|SetVisibility (Variables|Character|GetMesh) _returnvalue false))

(event OnGrabbed(HandbrakeGC)
  ;[1 1 1] Handbrake Control
  (Utilities|Time|SetTimerbyEvent (delegate Custom|MoveHandbrake) 0.01 true))

(event OnDropped(HandbrakeGC)
  ;[1 1 1] Handbrake Control
  (Class|KismetSystemLibrary|PauseTimer 0 "MoveHandbrake"))

(event OnGrabbed(ChainLeverRightGC)
  ;[1 1 1] ChainLeverRight Control
  (Utilities|Time|SetTimerbyEvent (delegate Custom|MoveChainLeverRight) 0.01 true))

(event OnDropped(ChainLeverRightGC)
  ;[1 1 1] ChainLeverRight Control
  (Class|KismetSystemLibrary|PauseTimer 0 "MoveChainLeverRight"))

(event OnGrabbed(ChainLeverLeftGC)
  ;[1 1 1] ChainLeverLeft Control
  (Utilities|Time|SetTimerbyEvent (delegate Custom|MoveChainLeverLeft) 0.01 true))

(event Custom|RotateWheel
  (bind _sm_steeringwheel (Variables|Default|GetSM_SteeringWheel))
  (bind _sm_steeringwheel_2 (Variables|Default|GetSM_SteeringWheel))
  (bind _direction (Variables|Default|GetDirection))
  (bind _returnvalue (Transformation|GetWorldLocation _sm_steeringwheel))
  (bind _relativerotation (Variables|/Script/Engine.SceneComponent|GetRelativeRotation _sm_steeringwheel_2))
  (bind _returnvalue_2 (Math|Float|MapRangeClamped (.roll _relativerotation) -9e+01 9e+01 -1.0 1.0))
  (bind _returnvalue_3 (* _returnvalue_2 _direction))
  ;[1 1 1] Steering Wheel Control
  (bind _mcloc (CallFunction|GetGrabbingMCLoc _returnvalue))
  (Transformation|SetRelativeRotation _sm_steeringwheel_2 (Math|Rotator|MakeRotator (Math|Float|Clamp(Float) (+ (.roll (Variables|/Script/Engine.SceneComponent|GetRelativeRotation _sm_steeringwheel_2)) (* (Math|Rotator|NormalizeAxis (Math|Vector|DotProduct (Math|Rotator|GetRotationXVector (Math|Rotator|FindLookatRotation _returnvalue _mcloc)) (Math|Vector|GetRightVector (Transformation|GetWorldRotation _sm_steeringwheel)))) 5e+01)) -9e+01 9e+01) 0.0 0.0) false false)
  (Class|ChaosVehicleMovementComponent|SetYawInput (Variables|Default|GetChaosWheeledVehicleMovement) _returnvalue_3)
  (Variables|Default|SetSteeringCache _returnvalue_3))

(event Custom|MoveDirectionLever
  (bind _sm_directionlever (Variables|Default|GetSM_DirectionLever))
  ;[1 1 1] Direction Lever Control
  (bind _newparam (CallFunction|CalcLeverAngle _sm_directionlever))
  (Transformation|SetRelativeRotation _sm_directionlever (Math|Rotator|MakeRotator 0.0 (Math|Float|Clamp(Float) _newparam -2e+01 2e+01) 0.0) false false)
  (if (Variables|Default|GetClutch)
    _
    (elif (!= (Variables|Default|GetDirection) (Math|Float|Round (Math|Float|MapRangeClamped (Math|Float|Clamp(Float) _newparam -2e+01 2e+01) -2e+01 2e+01 1.0 -1.0)))
      (Math|Integer|IncrementInt (Variables|Default|GetErrors)
        (:%20%20
          (CallFunction|TestAlive)))))
  (Variables|Default|SetDirection (Math|Float|Round (Math|Float|MapRangeClamped (Math|Float|Clamp(Float) _newparam -2e+01 2e+01) -2e+01 2e+01 1.0 -1.0)))
  (if (> (Variables|Default|GetGear) 4)
    (if (< (Variables|Default|GetDirection) 0)
      (CallFunction|KillTank)
      (else
        (CallFunction|SetGear :!label _label)))
    (else
      (goto _label))))

(event Custom|MoveHandbrake
  (bind _sm_handbrake (Variables|Default|GetSM_Handbrake))
  ;[1 1 1] Handbrake Control
  (bind _newparam (CallFunction|CalcLeverAngle _sm_handbrake))
  (Transformation|SetRelativeRotation _sm_handbrake (Math|Rotator|MakeRotator 0.0 (Math|Float|Clamp(Float) _newparam -2e+01 0.0) 0.0) false false)
  (Class|ChaosVehicleMovementComponent|SetHandbrakeInput (Variables|Default|GetChaosWheeledVehicleMovement) (> (Math|Float|MapRangeClamped (Math|Float|Clamp(Float) _newparam -2e+01 0.0) -2e+01 0.0 0.0 1.0) 0.9))
  (bind _output_get (Variables|Default|SetHB (> (Math|Float|MapRangeClamped (Math|Float|Clamp(Float) _newparam -2e+01 0.0) -2e+01 0.0 0.0 1.0) 0.9)))
  (if (not _output_get)
    (Class|ChaosVehicleMovementComponent|SetYawInput (Variables|Default|GetChaosWheeledVehicleMovement) (Variables|Default|GetSteeringCache))))

(event Custom|MoveChainLeverRight
  (bind _sm_chainleverright (Variables|Default|GetSM_ChainLeverRight))
  ;[1 1 1] ChainLeverRight Control
  (bind _newparam (CallFunction|CalcLeverAngle _sm_chainleverright))
  (Transformation|SetRelativeRotation _sm_chainleverright (Math|Rotator|MakeRotator 0.0 (Math|Float|Clamp(Float) _newparam -3e+01 0.0) 0.0) false false)
  (if (Variables|Default|GetHBRight)
    (if (not (> (Math|Float|MapRangeClamped (Math|Float|Clamp(Float) _newparam -3e+01 0.0) -3e+01 0.0 0.0 1.0) 0.9))
      (CallFunction|ReleaseChainBrake false))
    (elif (> (Math|Float|MapRangeClamped (Math|Float|Clamp(Float) _newparam -3e+01 0.0) -3e+01 0.0 0.0 1.0) 0.9)
      (CallFunction|SetChainBrake false))))

(event Custom|MoveGearLever
  (bind _sm_gearlever (Variables|Default|GetSM_GearLever))
  ;[1 1 1] Gear Lever Control
  (bind _newparam (CallFunction|CalcLeverAngle _sm_gearlever))
  (if (< (Variables|Default|GetDirection) 0)
    (Transformation|SetRelativeRotation _sm_gearlever (Math|Rotator|MakeRotator 0.0 (Math|Float|Clamp(Float) _newparam 4e+01 7e+01) 0.0) false false)
    (Variables|Default|SetNewGear (Math|Float|Round (Math|Float|MapRangeClamped (Math|Float|Clamp(Float) _newparam 4e+01 7e+01) 4e+01 7e+01 4.0 1.0)))
    (else
      (Transformation|SetRelativeRotation _sm_gearlever (Math|Rotator|MakeRotator 0.0 (Math|Float|Clamp(Float) _newparam 0.0 7e+01) 0.0) false false)
      (Variables|Default|SetNewGear (Math|Float|Round (Math|Float|MapRangeClamped (Math|Float|Clamp(Float) _newparam 0.0 7e+01) 0.0 7e+01 8.0 1.0)))))
  (if (Variables|Default|GetClutch)
    _
    (elif (!= (Variables|Default|GetNewGear) (Variables|Default|GetGear))
      (Math|Integer|IncrementInt (Variables|Default|GetErrors)
        (:%20%20
          (CallFunction|TestAlive)))))
  (Variables|Default|SetGear (Variables|Default|GetNewGear))
  (CallFunction|SetGear))

(event Custom|MoveChainLeverLeft
  (bind _sm_chainleverleft (Variables|Default|GetSM_ChainLeverLeft))
  ;[1 1 1] ChainLeverLeft Control
  (bind _newparam (CallFunction|CalcLeverAngle _sm_chainleverleft))
  (Transformation|SetRelativeRotation _sm_chainleverleft (Math|Rotator|MakeRotator 0.0 (Math|Float|Clamp(Float) _newparam -3e+01 0.0) 0.0) false false)
  (if (Variables|Default|GetHBLeft)
    (if (not (> (Math|Float|MapRangeClamped (Math|Float|Clamp(Float) _newparam -3e+01 0.0) -3e+01 0.0 0.0 1.0) 0.9))
      (CallFunction|ReleaseChainBrake true))
    (elif (> (Math|Float|MapRangeClamped (Math|Float|Clamp(Float) _newparam -3e+01 0.0) -3e+01 0.0 0.0 1.0) 0.9)
      (CallFunction|SetChainBrake true))))

(event EventTick
  (params (DeltaSeconds :type Float%20%28single-precision%29))
  (bind _chaoswheeledvehiclemovement (Variables|Default|GetChaosWheeledVehicleMovement))
  (bind _hbleft (Variables|Default|GetHBLeft))
  (bind _returnvalue (Vehicle|GetForwardSpeed _chaoswheeledvehiclemovement))
  ;[1 1 1] No rotation while standing
  (CallFunction|UpdateDisplay _returnvalue (Class|ChaosWheeledVehicleMovementComponent|GetEngineRotationSpeed _chaoswheeledvehiclemovement))
  (CallFunction|RotateWidgetstoCamera)
  (if (Variables|Default|GetHB)
    (Class|ChaosVehicleMovementComponent|SetYawInput _chaoswheeledvehiclemovement 0.0 :!label _label)
    (elif (not (> (Math|Float|Absolute(Float) _returnvalue) 5.0))
      (if (Variables|Default|GetHBRight)
        (if _hbleft
          (goto _label)
          (else
            _))
        (elif _hbleft
          _
          (else
            (goto _label))))
      (if (not (Variables|Default|GetDoAccelerate))
        (goto _label)))))

(fn ConstructionScript)

(fn GetGrabbingMCLoc
  (params (GrabbedLoc :type Vector))
  (bind _asvrpawn (Utilities|Casting|CastToVRPawn (Game|Player|GetPlayerPawn 0)))
  (if (< (Math|Vector|VectorLength (- (Transformation|GetWorldLocation (Variables|/Game/VRTemplate/Blueprints/VRPawn.VRPawn_C|GetMotionControllerRightGrip _asvrpawn)) GrabbedLoc)) (Math|Vector|VectorLength (- (Transformation|GetWorldLocation (Variables|/Game/VRTemplate/Blueprints/VRPawn.VRPawn_C|GetMotionControllerLeftGrip _asvrpawn)) GrabbedLoc)))
    (return (Transformation|GetWorldLocation (Variables|/Game/VRTemplate/Blueprints/VRPawn.VRPawn_C|GetMotionControllerRightGrip _asvrpawn)))
    (else
      (return (Transformation|GetWorldLocation (Variables|/Game/VRTemplate/Blueprints/VRPawn.VRPawn_C|GetMotionControllerLeftGrip _asvrpawn))))))

(fn Accelerate
  (params (InputValue :type Float%20%28double-precision%29))
  (bind _rotationspeed (LocalVariables|GetRotationSpeed))
  (bind _chaoswheeledvehiclemovement (Variables|Default|GetChaosWheeledVehicleMovement))
  (bind _direction (Variables|Default|GetDirection))
  (bind _returnvalue (* _rotationspeed _direction))
  (Variables|Default|SetDoAccelerate true)
  (Transformation|SetRelativeLocation (Variables|Default|GetSM_GasPedal) (+ (LocalVariables|GetGasPedalLoc) (* (LocalVariables|GetGasPedalOffset) InputValue)) false false)
  (if (Variables|Default|GetAlive)
    (if (not (Variables|Default|GetClutch))
      ;[1 1 1] Drehung bei angezogener Kettenbremse
      (if (Variables|Default|GetHBLeft)
        (if (not (Variables|Default|GetHBRight))
          (Class|ChaosVehicleMovementComponent|SetYawInput _chaoswheeledvehiclemovement (* _returnvalue -1.0)))
        (elif (Variables|Default|GetHBRight)
          (Class|ChaosVehicleMovementComponent|SetYawInput _chaoswheeledvehiclemovement _returnvalue)
          (else
            ;[1 1 1] Beschleunigung
            (if (!= _direction 0)
              (Class|ChaosVehicleMovementComponent|SetThrottleInput _chaoswheeledvehiclemovement InputValue)
              (else
                (Class|ChaosVehicleMovementComponent|SetThrottleInput _chaoswheeledvehiclemovement 0.0)))))))
    (else
      (Class|ChaosVehicleMovementComponent|SetThrottleInput (Variables|Default|GetChaosWheeledVehicleMovement) 0.0))))

(fn Brake
  (params (InputValue :type Float%20%28double-precision%29))
  (Transformation|SetRelativeLocation (Variables|Default|GetSM_BrakePedal) (+ (LocalVariables|GetBrakePedalLoc) (* (LocalVariables|GetBrakePedalOffset) InputValue)) false false)
  (Class|ChaosVehicleMovementComponent|SetBrakeInput (Variables|Default|GetChaosWheeledVehicleMovement) InputValue))

(fn CalcLeverAngle
  (params (Lever :type Scene%20Component%20Object%20Reference))
  (bind _returnvalue (Transformation|GetWorldLocation Lever))
  (bind _mcloc (CallFunction|GetGrabbingMCLoc _returnvalue))
  (return (+ (.pitch (Variables|/Script/Engine.SceneComponent|GetRelativeRotation Lever)) (* 1e+01 (Math|Vector|DotProduct (Math|Rotator|GetRotationXVector (Math|Rotator|FindLookatRotation _returnvalue _mcloc)) (* (Math|Vector|GetForwardVector (Transformation|GetWorldRotation Lever)) -1.0))))))

(fn SetGear
  (Class|ChaosVehicleMovementComponent|SetTargetGear (Variables|Default|GetChaosWheeledVehicleMovement) (* (Variables|Default|GetDirection) (Variables|Default|GetGear)) false))

(fn PressClutch
  (params (Input%20Value :type Float%20%28double-precision%29))
  (Transformation|SetRelativeLocation (Variables|Default|GetSM_ClutchPedal) (+ (LocalVariables|GetClutchPedalLoc) (* (LocalVariables|GetClutchPedalOffset) Input%20Value)) false false)
  (Variables|Default|SetClutch true))

(fn ReleaseClutch
  (Variables|Default|SetClutch false))

(fn TestAlive
  (if (>= (Variables|Default|GetErrors) (Math|Random|RandomIntegerinRange 15 500))
    (CallFunction|KillTank)))

(fn UpdateDisplay
  (params (Speed :type Float%20%28double-precision%29) (RPM :type Float%20%28double-precision%29))
  (Transformation|SetRelativeRotation (Variables|Default|GetSM_SpeedPointer) (Math|Rotator|MakeRotator 0.0 0.0 (Math|Float|MapRangeClamped (Math|Float|Absolute(Float) Speed) 0.0 1.4e+03 -3e+01 2.1e+02)) false false)
  (Transformation|SetRelativeRotation (Variables|Default|GetSM_RPMPointer) (Math|Rotator|MakeRotator 0.0 0.0 (Math|Float|MapRangeClamped (Math|Float|Absolute(Float) RPM) 0.0 5e+03 -3e+01 2.1e+02)) false false))

(fn EndAccelerate
  (bind _chaoswheeledvehiclemovement (Variables|Default|GetChaosWheeledVehicleMovement))
  (bind _hbleft (Variables|Default|GetHBLeft))
  (Variables|Default|SetDoAccelerate false)
  (Class|ChaosVehicleMovementComponent|SetThrottleInput _chaoswheeledvehiclemovement 0.0)
  (if (Variables|Default|GetHBRight)
    (if (not _hbleft)
      (Class|ChaosVehicleMovementComponent|SetYawInput _chaoswheeledvehiclemovement 0.0 :!label _label))
    (elif _hbleft
      (goto _label))))

(fn GetGrabbingMC
  (params (GrabbedLoc :type Vector))
  (bind _asvrpawn (Utilities|Casting|CastToVRPawn (Game|Player|GetPlayerPawn 0)))
  (if (< (Math|Vector|VectorLength (- (Transformation|GetWorldLocation (Variables|/Game/VRTemplate/Blueprints/VRPawn.VRPawn_C|GetMotionControllerRightGrip _asvrpawn)) GrabbedLoc)) (Math|Vector|VectorLength (- (Transformation|GetWorldLocation (Variables|/Game/VRTemplate/Blueprints/VRPawn.VRPawn_C|GetMotionControllerLeftGrip _asvrpawn)) GrabbedLoc)))
    (return (Variables|/Game/VRTemplate/Blueprints/VRPawn.VRPawn_C|GetMotionControllerRightGrip _asvrpawn))
    (else
      (return (Variables|/Game/VRTemplate/Blueprints/VRPawn.VRPawn_C|GetMotionControllerLeftGrip _asvrpawn)))))

(fn ReleaseChainBrake
  (params (IsHBLeft :type Boolean))
  (if IsHBLeft
    (Variables|Default|SetHBLeft false)
    (else
      (Variables|Default|SetHBRight false)))
  (if (not (Variables|Default|GetHB))
    (Class|ChaosVehicleMovementComponent|SetHandbrakeInput (Variables|Default|GetChaosWheeledVehicleMovement) false)
    (Class|ChaosVehicleMovementComponent|SetYawInput (Variables|Default|GetChaosWheeledVehicleMovement) (Variables|Default|GetSteeringCache))))

(fn SetChainBrake
  (params (IsHBLeft :type Boolean))
  (if (>= (Math|Float|Absolute(Float) (Vehicle|GetForwardSpeed (Variables|Default|GetChaosWheeledVehicleMovement))) 5e+01)
    (CallFunction|KillTank))
  ;[1 1 1] Prüfung, ob die andere Kettenbremse schon angezogen ist und wenn nötig aktiveieren der Handbremse
  (if IsHBLeft
    (LocalVariables|SetotherHB (Variables|Default|GetHBRight))
    (Variables|Default|SetHBLeft true)
    (else
      (LocalVariables|SetotherHB (Variables|Default|GetHBLeft))
      (Variables|Default|SetHBRight true)))
  (if (LocalVariables|GetotherHB)
    (Class|ChaosVehicleMovementComponent|SetHandbrakeInput (Variables|Default|GetChaosWheeledVehicleMovement) true)))

(fn KillTank
  (Variables|Default|SetAlive false)
  (Rendering|Material|SetMaterial (Variables|Default|GetSM_WarningLight) 0 "/Game/Panzersim/Vehicle/Materials/M_red_lighting.M_red_lighting")
  (Rendering|Components|Light|SetIntensity (Variables|Default|GetPL_WarningLight) 1e+02)
  (Audio|PlaySound2D "/Game/Panzersim/Sounds/Explosion_Cue.Explosion_Cue" 1.0 1.0 0.0 0 0))

(fn SetSketchbookVisibility
  (bind _output_get (Variables|Default|SetSketchbookIsGrabbed (not (Variables|Default|GetSketchbookIsGrabbed))))
  (Rendering|SetVisibility (Variables|Default|GetBP_Sketchfab) (not _output_get) true))

(fn ShowContolNumbers
  (params (Visibility :type Boolean))
  (Rendering|SetVisibility (Variables|Default|GetW_Count_Display) Visibility false)
  (Rendering|SetVisibility (Variables|Default|GetW_Count_ClutchPedal) Visibility false)
  (Rendering|SetVisibility (Variables|Default|GetW_Count_BrakePedal) Visibility false)
  (Rendering|SetVisibility (Variables|Default|GetW_Count_CommanderSight) Visibility false)
  (Rendering|SetVisibility (Variables|Default|GetW_Count_GasPedal) Visibility false)
  (Rendering|SetVisibility (Variables|Default|GetW_Count_DirectionLever) Visibility false)
  (Rendering|SetVisibility (Variables|Default|GetW_Count_Handbrake) Visibility false)
  (Rendering|SetVisibility (Variables|Default|GetW_Count_GearLever) Visibility false)
  (Rendering|SetVisibility (Variables|Default|GetW_Count_SteeringWheel) Visibility false)
  (Rendering|SetVisibility (Variables|Default|GetW_Count_ChainLeverLeft) Visibility false)
  (Rendering|SetVisibility (Variables|Default|GetW_Count_ChainLeverRight) Visibility false))

(fn RotateWidgetstoCamera
  (CallFunction|RotateWidgetComponenttoCamera (Variables|Default|GetW_Count_Display))
  (CallFunction|RotateWidgetComponenttoCamera (Variables|Default|GetW_Count_GasPedal))
  (CallFunction|RotateWidgetComponenttoCamera (Variables|Default|GetW_Count_BrakePedal))
  (CallFunction|RotateWidgetComponenttoCamera (Variables|Default|GetW_Count_ClutchPedal))
  (CallFunction|RotateWidgetComponenttoCamera (Variables|Default|GetW_Count_CommanderSight))
  (CallFunction|RotateWidgetComponenttoCamera (Variables|Default|GetW_Count_SteeringWheel))
  (CallFunction|RotateWidgetComponenttoCamera (Variables|Default|GetW_Count_Handbrake))
  (CallFunction|RotateWidgetComponenttoCamera (Variables|Default|GetW_Count_DirectionLever))
  (CallFunction|RotateWidgetComponenttoCamera (Variables|Default|GetW_Count_ChainLeverLeft))
  (CallFunction|RotateWidgetComponenttoCamera (Variables|Default|GetW_Count_GearLever))
  (CallFunction|RotateWidgetComponenttoCamera (Variables|Default|GetW_Count_ChainLeverRight)))

(fn RotateWidgetComponenttoCamera
  (params (Component :type Widget%20Component%20Object%20Reference))
  (Transformation|SetWorldRotation Component (Math|Rotator|FindLookatRotation (Transformation|GetWorldLocation Component) (Camera|GetCameraLocation (Game|GetPlayerCameraManager 0))) false false))